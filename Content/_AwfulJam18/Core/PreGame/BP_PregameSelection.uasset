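; BP_PregameSelection is a pregame selection indicator that displays a dog mesh with a selector material when flagged as Clicked.
; Its construction script applies DogMesh and MeshScale, overrides every material slot with M_Selector, then sets vector and depth parameters on the materials.
; When Clicked is false, the script destroys the arrow and skeletal mesh components.
; The event graph holds no active logic.
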(event EventBeginPlay)

(event Collision|EventActorBeginOverlap
  (params (OtherActor :type Actor%20Object%20Reference)))

(event EventTick
  (params (DeltaSeconds :type Float%20%28single-precision%29)))

(fn ConstructionScript
  (bind _skeletalmesh (Variables|Default|GetSkeletalMesh))
  (if (Variables|Default|Getclicked)
    (Class|SkinnedMeshComponent|SetSkeletalMesh _skeletalmesh (Variables|Default|GetdogMesh) true)
    (Transformation|SetWorldScale3D _skeletalmesh (Math|Conversions|ToVector(Float) (Variables|Default|GetmeshScale)))
    (for _array_element (Class|MeshComponent|GetMaterialSlotNames _skeletalmesh)
      (Rendering|Material|SetMaterialbyName _skeletalmesh _array_element "/Game/_AwfulJam18/Core/PreGame/M_Selector.M_Selector")
      (Rendering|Material|SetVectorParameterValueonMaterials _skeletalmesh "None" "1.000000,0.000000,1.000000")
      (Rendering|Material|SetScalarParameterValueonMaterials _skeletalmesh "depth" 2.0))
    (else
      (Components|DestroyComponent (Variables|Default|GetArrow)))))