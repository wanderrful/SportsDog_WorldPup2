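; Pre-game game mode for arranging the player's dog team before a match, judging by its selection, preview and save logic.
; BeginPlay binds hover and click events on every dog and collects team 0's dogs plus a goalkeeper.
; Hover and click spawn selection markers; Tick traces under the cursor to place a ghost mesh and stretched arrow from the selected dog.
; Saving passes position and breed maps, keyed by player ID, to the GameInstance, then begins the match.
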(event Custom|CustomEvent_0
  (params (TouchedComponent :type Primitive%20Component%20Object%20Reference) (ButtonPressed :type Key%20Structure))
  ;[1 1 1] Click On Dog
  (bind _asbp_base_dog (Utilities|Casting|CastToBP_Base_Dog (Components|GetOwner TouchedComponent)))
  (Utilities|FlowControl|Delay 0.2)
  (bind _output_get (Variables|Default|SetCurrentlySelectedDog _asbp_base_dog))
  (Default|DogThings _output_get)
  (Utilities|Casting|CastToBP_PreGame_HUD (HUD|GetHUD (Game|GetPlayerController 0)))
  (Utilities|IsValid (Variables|Default|GetcurrentClickCircle)
    (:Is%20Valid
      (Actor|DestroyActor (Variables|Default|GetcurrentClickCircle)))
    (:Is%20Not%20Valid
      _))
  (bind _returnvalue (Game|SpawnActorfromClass "/Game/_AwfulJam18/Core/PreGame/BP_PregameSelection.BP_PregameSelection_C" (Math|Conversions|ToTransform(Vector) (Math|Vector|ProjectVectorontoPlane (Transformation|GetActorLocation _output_get) "0, 0,1.000000")) "Undefined" 0 true (Variables|/Script/Engine.SkinnedMeshComponent|GetSkeletalMesh (Variables|/Script/Engine.Character|GetMesh _output_get)) (* (Variables|/Game/_AwfulJam18/Characters/BP_Base_Dog.BP_Base_Dog_C|GetdogMeshScale _output_get) 2.0) 0))
  (Variables|Default|SetcurrentClickCircle _returnvalue)
  (Rendering|Material|SetVectorParameterValueonMaterials (Variables|/Game/_AwfulJam18/Core/PreGame/BP_PregameSelection.BP_PregameSelection_C|GetBase _returnvalue) "None" "1.000000, 0, 0")
  (Rendering|Material|SetScalarParameterValueonMaterials (Variables|/Game/_AwfulJam18/Core/PreGame/BP_PregameSelection.BP_PregameSelection_C|GetBase _returnvalue) "depth" 2.0))

(event Custom|CustomEvent_1
  (params (TouchedComponent :type Primitive%20Component%20Object%20Reference))
  ;[1 1 1] Mouse Over Dog
  (bind _asbp_base_dog (Utilities|Casting|CastToBP_Base_Dog (Components|GetOwner TouchedComponent)))
  (bind _returnvalue (Game|SpawnActorfromClass "/Game/_AwfulJam18/Core/PreGame/BP_PregameSelection.BP_PregameSelection_C" (Math|Conversions|ToTransform(Vector) (Math|Vector|ProjectVectorontoPlane (Transformation|GetActorLocation _asbp_base_dog) "0, 0,1.000000")) "Undefined" 0 false (Variables|/Script/Engine.SkinnedMeshComponent|GetSkeletalMesh (Variables|/Script/Engine.Character|GetMesh _asbp_base_dog)) (Variables|/Game/_AwfulJam18/Characters/BP_Base_Dog.BP_Base_Dog_C|GetdogMeshScale _asbp_base_dog) 0)))

(event Custom|CustomEvent_2
  (params (TouchedComponent :type Primitive%20Component%20Object%20Reference))
  ;[1 1 1] Mouse Over Dog
  (Actor|DestroyActor (stale Custom|CustomEvent_1 _returnvalue)))

(event Custom|eh_OnSaveDogPositionsAndBeginMatch
  (bind _asbp_awful_jam_18_gi (Utilities|Casting|CastToBP_AwfulJam18_GI (Game|GetGameInstance)))
  (Variables|/Game/_AwfulJam18/Core/BP_AwfulJam18_GI.BP_AwfulJam18_GI_C|SetChosenStartingPositions _asbp_awful_jam_18_gi (CallFunction|FnGetDogPositionMap))
  (Variables|/Game/_AwfulJam18/Core/BP_AwfulJam18_GI.BP_AwfulJam18_GI_C|SetChosenDogBreeds _asbp_awful_jam_18_gi (CallFunction|FnGetDogBreedMap))
  (Default|EhonBeginMatch _asbp_awful_jam_18_gi))

(event EventBeginPlay
  (|CallParentFunction)
  (Utilities|FlowControl|Sequence
    (:then_1
      (bind _outactors (Actor|GetAllActorsOfClass "/Game/_AwfulJam18/Characters/BP_Base_Dog.BP_Base_Dog_C"))
      (for _array_element _outactors
        (Utilities|FlowControl|Sequence
          (:then_0
            (EventDispatchers|BindEventtoOnBeginCursorOver (Variables|/Script/Engine.Character|GetCapsuleComponent _array_element) (delegate Custom|CustomEvent_1))
            (EventDispatchers|BindEventtoOnEndCursorOver (Variables|/Script/Engine.Character|GetCapsuleComponent _array_element) (delegate Custom|CustomEvent_2))
            (EventDispatchers|BindEventtoOnClicked (Variables|/Script/Engine.Character|GetCapsuleComponent _array_element) (delegate Custom|CustomEvent_0)))
          (:then_1
            (if (and (== (Variables|/Game/_AwfulJam18/Characters/BP_Base_Dog.BP_Base_Dog_C|GetTeamID _array_element) 0) (Utilities|Enum|NotEqual(Enum) (Variables|/Game/_AwfulJam18/Characters/BP_Base_Dog.BP_Base_Dog_C|GetplayerRole _array_element) "NewEnumerator0"))
              (Utilities|Array|Add (Variables|Default|GetPlayerDogs) _array_element)
              (elif (not (Utilities|Enum|NotEqual(Enum) (Variables|/Game/_AwfulJam18/Characters/BP_Base_Dog.BP_Base_Dog_C|GetplayerRole _array_element) "NewEnumerator0"))
                (Variables|Default|SetGoalkeeperDog _array_element)))))))))

(event EventTick
  (params (DeltaSeconds :type Float%20%28single-precision%29))
  (bind _returnvalue (Game|GetPlayerController 0))
  (bind _currentclickcircle (Variables|Default|GetcurrentClickCircle))
  (bind _returnvalue_2 (Transformation|GetActorLocation _currentclickcircle))
  (bind (_worldlocation _worlddirection) (Game|Player|ConvertMouseLocationToWorldSpace _returnvalue))
  (bind _arrow (Variables|/Game/_AwfulJam18/Core/PreGame/BP_PregameSelection.BP_PregameSelection_C|GetArrow _currentclickcircle))
  (bind _skeletalmesh (Variables|/Game/_AwfulJam18/Core/PreGame/BP_PregameSelection.BP_PregameSelection_C|GetSkeletalMesh _currentclickcircle))
  ;[1 1 1] Arrow + Dog Position preview
  (if (Utilities|IsValid _currentclickcircle)
    (bind (_outhit _returnvalue_3) (Collision|LineTraceForObjects _worldlocation (+ _worldlocation (* _worlddirection 111111.0)) (Utilities|Array|MakeArray "ObjectTypeQuery1" "ObjectTypeQuery4") false 0 "None"))
    (if _returnvalue_3
      (Utilities|Casting|CastToBP_Base_Dog (.HitActor (Collision|BreakHitResult _outhit))
        (:then
          (Development|SetHiddeninGame _skeletalmesh true false)
          (Development|SetHiddeninGame _arrow true false))
        (:CastFailed
          (Development|SetHiddeninGame _skeletalmesh false false)
          (Development|SetHiddeninGame _arrow false false)
          (Transformation|SetWorldLocationAndRotation _skeletalmesh (.Location (Collision|BreakHitResult _outhit)) "0,90.000000, 0" false false)
          (Transformation|SetWorldTransform _arrow (Math|Transform|MakeTransform _returnvalue_2 (Math|Rotator|FindLookatRotation _returnvalue_2 (.Location (Collision|BreakHitResult _outhit))) (Math|Vector|MakeVector (/ (Math|Vector|VectorLength (- (.Location (Collision|BreakHitResult _outhit)) _returnvalue_2)) 1.6e+03) 0.6 0.6)) false false))))))

(fn ConstructionScript
  (|CallParentFunction))

(fn FnFindDogbyName
  (params (InputPin :type String))
  (bind _array_element (Utilities|Array|ForEachLoopwithBreak (Variables|Default|GetPlayerDogs) :!label _label)
    (:LoopBody
      (if (Utilities|Enum|Equal(Enum) InputPin (Utilities|GetDisplayName _array_element))
        (LocalVariables|SetChosenDog _array_element)
        (goto _label Break)))
    (:Completed
      (return (LocalVariables|GetChosenDog)))))

(fn FnGetDogPositionMap
  (Utilities|Array|Add (Variables|Default|GetPlayerDogs) (Variables|Default|GetGoalkeeperDog))
  (for _array_element (Variables|Default|GetPlayerDogs)
    (Utilities|Map|Add (LocalVariables|Gett_Positions) (Variables|/Game/_AwfulJam18/Characters/BP_Base_Dog.BP_Base_Dog_C|GetPlayerID _array_element) (Math|Conversions|ToVector2D(Vector) (Transformation|GetActorLocation _array_element)))
    (Development|PrintString (Utilities|String|ToString(Vector2d) (Math|Conversions|ToVector2D(Vector) (Transformation|GetActorLocation _array_element))) false true "(R=0.935651,G=0.000000,B=1.000000,A=1.000000)"))
  (return (LocalVariables|Gett_Positions)))

(fn FnGetDogBreedMap
  (for _array_element (Variables|Default|GetPlayerDogs)
    (Utilities|Map|Add (LocalVariables|Gett_Positions) (Variables|/Game/_AwfulJam18/Characters/BP_Base_Dog.BP_Base_Dog_C|GetPlayerID _array_element) (Variables|/Game/_AwfulJam18/Characters/BP_Base_Dog.BP_Base_Dog_C|GetAssignedBreed _array_element)))
  (return (LocalVariables|Gett_Positions)))