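; Pre-game player controller that orders the selected dog around and pans the camera.
; A move click traces under the cursor and, unless it hits a dog, sends the game mode's selected dog there by AI MoveTo, removing the selection actor and clearing the selection.
; Tick pans the view target from keys or screen edges within fixed XY bounds.
; Escape input toggles the menu through a cast to BP_Game_GM.
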(event EventTick
  (params (DeltaSeconds :type Float%20%28single-precision%29))
  (Game|Camera|FnHandleCameraPanning))

(event Input|ActionEvents|InputActionToggleEscapeMenu
  (params (Key :type Key%20Structure))
  (bind _returnvalue (Game|GetGameMode))
  (bind (_asbp_game_gm _bsuccess) (Utilities|Casting|CastToBP_Game_GM _returnvalue))
  (:Pressed
    (if _bsuccess
      (Default|EhonToggleEscapeMenu (Variables|/Game/_AwfulJam18/Core/BP_Game_GM.BP_Game_GM_C|GetUI_EscapeMenu _asbp_game_gm)))))

(event Input|ActionEvents|InputActionIssueMoveOrder
  (params (Key :type Key%20Structure))
  (bind (_locationx _locationy) (Game|Player|GetMousePosition))
  (bind _self self)
  (bind (_worldposition _worlddirection) (Class|GameplayStatics|DeprojectScreentoWorld _self (Math|Vector2D|MakeVector2D _locationx _locationy)))
  (:Pressed
    (bind (_outhit _returnvalue) (Collision|LineTraceForObjects (+ _worldposition (* _worlddirection 1e+02)) (+ _worldposition (* _worlddirection 5e+04)) (Utilities|Array|MakeArray "ObjectTypeQuery1" "ObjectTypeQuery4") false (Utilities|Array|MakeArray (Pawn|GetControlledPawn) (Pawn|GetViewTarget)) "None"))
    (if _returnvalue
      (Utilities|Casting|CastToBP_Base_Dog (.hitactor _outhit)
        (:then)
        (:CastFailed
          (Game|AI|FnIssueMoveOrder (Math|Vector|MakeVector (.X (Math|Vector|BreakVector (.location _outhit))) (.Y (Math|Vector|BreakVector (.location _outhit))) 0.0)))))))

(event Input|ActionEvents|InputActionCameraPanManualUP
  (params (Key :type Key%20Structure))
  (:Pressed
    (Variables|Game|Camera|SetbShouldPanUp true))
  (:Released
    (Variables|Game|Camera|SetbShouldPanUp false)))

(event Input|ActionEvents|InputActionCameraPanManualDOWN
  (params (Key :type Key%20Structure))
  (:Pressed
    (Variables|Game|Camera|SetbShouldPanDown true))
  (:Released
    (Variables|Game|Camera|SetbShouldPanDown false)))

(event Input|ActionEvents|InputActionCameraPanManualLEFT
  (params (Key :type Key%20Structure))
  (:Pressed
    (Variables|Game|Camera|SetbShouldPanLeft true))
  (:Released
    (Variables|Game|Camera|SetbShouldPanLeft false)))

(event Input|ActionEvents|InputActionCameraPanManualRIGHT
  (params (Key :type Key%20Structure))
  (:Pressed
    (Variables|Game|Camera|SetbShouldPanRight true))
  (:Released
    (Variables|Game|Camera|SetbShouldPanRight false)))

(fn ConstructionScript)

(fn FnIssueMoveOrder
  (params (Destination :type Vector))
  (bind _asbp_pre_game_gm (Utilities|Casting|CastToBP_PreGame_GM (Game|GetGameMode))
    (:then
      (bind _currentlyselecteddog (Variables|/Game/_AwfulJam18/Core/PreGame/BP_PreGame_GM.BP_PreGame_GM_C|GetCurrentlySelectedDog _asbp_pre_game_gm)
        (:then
          (Default|DogThings _currentlyselecteddog)
          (AI|Navigation|MovetoLocation (AI|GetAIController _currentlyselecteddog) Destination 5e+01 true true false)
          (bind _outactors (Actor|GetAllActorsOfClass "/Game/_AwfulJam18/Core/PreGame/BP_PregameSelection.BP_PregameSelection_C"))
          (if (> (Utilities|Array|Length _outactors) 0)
            (Actor|DestroyActor (Utilities|Array|Get(acopy) _outactors))
            (bind _asbp_pre_game_gm_2 (Utilities|Casting|CastToBP_PreGame_GM (Game|GetGameMode))
              (:then
                (Variables|/Game/_AwfulJam18/Core/PreGame/BP_PreGame_GM.BP_PreGame_GM_C|SetCurrentlySelectedDog _asbp_pre_game_gm_2 0))
              (:CastFailed
                _))))
        (:else
          (Development|PrintString "* NO DOG SELECTED" :!label _label))))
    (:CastFailed
      (goto _label)))
  (return))

(fn FnHandleCameraPanning
  (bind _returnvalue (Pawn|GetViewTarget))
  (bind _locationy (Game|Player|GetMousePosition))
  (bind _returnvalue_2 (Viewport|GetViewportSize))
  (bind _locationx (Game|Player|GetMousePosition))
  (bind _returnvalue_3 (Viewport|GetViewportSize))
  (Utilities|FlowControl|Sequence
    (:then_0
      (Utilities|FlowControl|Sequence
        (:then_0
          (if (or (Variables|Game|Camera|GetbShouldPanLeft) (and (!= _locationx 0.0) (|((A/B)<0.030000) _locationx (.x _returnvalue_3))))
            (Variables|Default|SetCameraOffset (+ (Variables|Default|GetCameraOffset) (Math|Vector|MakeVector (Variables|Default|GetCameraMovementSpeed) 0.0 0.0)))))
        (:then_1
          (if (or (Variables|Game|Camera|GetbShouldPanRight) (|((A/B)>0.970000) _locationx (.x _returnvalue_3)))
            (Variables|Default|SetCameraOffset (+ (Variables|Default|GetCameraOffset) (Math|Vector|MakeVector (* (Variables|Default|GetCameraMovementSpeed) -1.0) 0.0 0.0)))))
        (:then_2
          (if (or (Variables|Game|Camera|GetbShouldPanUp) (and (!= _locationy 0.0) (|((A/B)<0.030000) _locationy (.y _returnvalue_2))))
            (Variables|Default|SetCameraOffset (+ (Variables|Default|GetCameraOffset) (Math|Vector|MakeVector 0.0 (Variables|Default|GetCameraMovementSpeed) 0.0)))))
        (:then_3
          (if (or (Variables|Game|Camera|GetbShouldPanDown) (|((A/B)>0.970000) _locationy (.y _returnvalue_2)))
            (Variables|Default|SetCameraOffset (+ (Variables|Default|GetCameraOffset) (Math|Vector|MakeVector 0.0 (* (Variables|Default|GetCameraMovementSpeed) -1.0) 0.0)))))))
    (:then_1
      (Utilities|FlowControl|Sequence
        (:then_0
          (if (not (.bIsInBoundsX (Game|Camera|FnBIsPositioninBounds (+ (Variables|Default|GetCameraOffset) (Transformation|GetActorLocation _returnvalue)))))
            (Variables|Default|SetCameraOffset (Math|Vector|MakeVector 0.0 (.y (Variables|Default|GetCameraOffset)) 0.0))))
        (:then_1
          (if (not (.bIsInBoundsY (Game|Camera|FnBIsPositioninBounds (+ (Variables|Default|GetCameraOffset) (Transformation|GetActorLocation _returnvalue)))))
            (Variables|Default|SetCameraOffset (Math|Vector|MakeVector (.x (Variables|Default|GetCameraOffset)) 0.0 0.0))))
        (:then_2
          (Transformation|AddActorWorldOffset _returnvalue (Variables|Default|GetCameraOffset))
          (Variables|Default|SetCameraOffset "0, 0, 0"))))))

(fn FnBIsPositioninBounds
  (params (GivenPosition :type Vector))
  (return (and (< (.x GivenPosition) 4e+03) (> (.x GivenPosition) -4e+03)) (and (< (.y GivenPosition) 0.0) (> (.y GivenPosition) -5e+03))))