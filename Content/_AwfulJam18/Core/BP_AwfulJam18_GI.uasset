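; Game Instance for a dog-team tournament game, owning the bracket, breed and skill unlocks, and level travel.
; It shuffles DT_Teams into a slot-numbered bracket map, finds opponents by slot parity, and randomly resolves matches without the player.
; Wins advance the bracket and unlock the opponent's breed and skill, while losses flag a knockout.
; Only the game-beaten flag persists via SaveGame, granting the Golden Retriever on init and reset.
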(event Custom|eh_OnResetGame
  (Utilities|FlowControl|Sequence
    (:then_0
      (Variables|Game|Bracket|SetbJustBeatTheGame false) ; Reset any left-over stuff that might have existed from a previous play through!!
      (Variables|Game|Bracket|SetbWasKnockedOut false)
      (Utilities|Array|Clear (Variables|Game|Teams|GetUnlockedBreeds)) ; Reset the available dog breeds on Game Over!
      (Utilities|Array|Clear (Variables|Game|Teams|GetUnlockedSkills))
      (Utilities|Map|Clear (Variables|Game|Bracket|GetBracketStatus))
      (SaveGame|FnWriteSaveGameData))
    (:then_1
      (if (Variables|Game|GetbHasBeatenTheGameBefore) ; Unlock the Golden Retriever if eligible
        (bind _returnvalue (Utilities|GetDataTableRow "/Game/_AwfulJam18/Core/DT_Dogs.DT_Dogs" "retriever")
          (:then
            (Game|Teams|FnUnlockBreed _returnvalue)))))
    (:then_2
      (Game|Bracket|FnInitializeNewBracket) ; POLISH: Maybe we want to initialize a new bracket only if we click the New Game button? (for if we add savegame data)
      (CallFunction|EhonReturntoMainMenu))))

(event EventInit
  (Utilities|FlowControl|Sequence
    (:then_0
      (SaveGame|FnInitSaveGameData)
      (SaveGame|FnReadSaveGameData)
      (if (Variables|Game|GetbHasBeatenTheGameBefore) ; Unlock the Golden Retriever if eligible
        (bind _returnvalue (Utilities|GetDataTableRow "/Game/_AwfulJam18/Core/DT_Dogs.DT_Dogs" "retriever")
          (:then
            (Game|Teams|FnUnlockBreed _returnvalue)))))
    (:then_1
      (if (not (.ReturnValue (Utilities|Map|Find (Variables|Game|Bracket|GetBracketStatus) 9))) ; Is there a reason not to init a new bracket?
        (Game|Bracket|FnInitializeNewBracket) ; POLISH: Maybe we want to initialize a new bracket only if we click the New Game button? (for if we add savegame data)
      ))))

(event EventShutdown
  (SaveGame|FnWriteSaveGameData))

(event Custom|eh_OnBeginPreGame
  (if (not (Utilities|Text|TextIsEmpty (Utilities|Text|ToText(String) (.teamname (Variables|Game|Teams|GetChosenTeam)))))
    (Variables|Game|Teams|SetCurrentOpposingTeam (Game|Teams|FnGetNextOpponent))
    (bind _output_get (Variables|Default|Setmusictime (Class|GameplayStatics|GetAudioTimeSeconds)))
    (Game|OpenLevel(byName) (Variables|Game|GetPreGameMapName) true "?game=/Game/_AwfulJam18/Core/PreGame/BP_PreGame_GM.BP_PreGame_GM_C") ; This will take us to the PreGame mode!
    (Utilities|FlowControl|Delay 0.0)
    (Audio|PlaySound2D "/Game/Sound/MUSIC_LOOP2_Cue.MUSIC_LOOP2_Cue" 0.25 1.0 _output_get)))

(event Custom|eh_OnReturnToMainMenu
  (Game|OpenLevel(byName) "Startuplevel_Persistent") ; This will take us straight to the simluation
)

(event Custom|eh_OnProgressToBracket
  (Game|OpenLevel(byName) "Bracket")
  (Utilities|FlowControl|Delay 0.0)
  (Audio|PlaySound2D "/Game/Sound/MUSIC_LOOP2_Cue.MUSIC_LOOP2_Cue" 0.25))

(event Custom|eh_OnBeginMatch
  (Game|OpenLevel(byName) (Variables|Game|GetGameplayMapName)) ; This will take us straight to the simluation
)

(event Custom|eh_OnMatchCompleted
  (params (bPlayerWonTheMatch :type Boolean))
  (bind _currentopposingteam (Variables|Game|Teams|GetCurrentOpposingTeam))
  (Game|Match|FnGameShowNotification (select bPlayerWonTheMatch "YOU WIN" "YOU LOSE"))
  (Utilities|FlowControl|Delay 5.0)
  (if bPlayerWonTheMatch
    (Game|Bracket|FnProgresstoNextRound) ; TODO: after this, we want to return to the bracket for the player to review the tournament status and so that they can continue to the next PreGame!
    (bind _returnvalue (Utilities|GetDataTableRow "/Game/_AwfulJam18/Core/DT_Dogs.DT_Dogs" (.dog _currentopposingteam))
      (:then
        (Game|Teams|FnUnlockBreed _returnvalue) ; TODO: Polish-- add a UI notification that we unlocked a new dog breed!
        (Utilities|Array|AddUnique (Variables|Game|Teams|GetUnlockedSkills) (.skill _currentopposingteam))
        (SaveGame|FnWriteSaveGameData)
        (CallFunction|EhonProgresstoBracket) ; The Bracket level will take care of the game over state
      ))
    (else
      (Game|OpenLevel(byName) "Startuplevel_Persistent")
      (Variables|Game|Bracket|SetbWasKnockedOut true)
      (CallFunction|EhonProgresstoBracket) ; The Bracket level will take care of the game over state
    )))

(event Custom|eh_OnWonTheTournament
  (Variables|Game|Bracket|SetbJustBeatTheGame true)
  (Variables|Game|SetbHasBeatenTheGameBefore true))

(fn FnGetNewBracketData
  (bind _outrownames (DataTable|GetDataTableRowNames "/Game/_AwfulJam18/Core/DT_Teams.DT_Teams"))
  (bind _output_get (LocalVariables|Sett_Rows _outrownames))
  (Utilities|Array|Shuffle _output_get)
  (for (_array_element _array_index) (LocalVariables|Gett_Rows)
    (bind _returnvalue (Utilities|GetDataTableRow "/Game/_AwfulJam18/Core/DT_Teams.DT_Teams" _array_element)
      (:then
        (Utilities|Map|Add (LocalVariables|Gett_BracketData) (+ _array_index 1) _returnvalue))))
  (return (LocalVariables|Gett_BracketData)))

(fn FnInitializeNewBracket
  (Variables|Game|Bracket|SetBracketStatus (Game|Bracket|FnGetNewBracketData)))

(fn FnResolveMatch
  (params (Team1 :type Integer) (Team2 :type Integer))
  (bind _id (Game|Bracket|FnGetPlayerTeamBracketID))
  (Utilities|FlowControl|Sequence
    (:then_0
      (if (== Team1 _id)
        (return Team1)))
    (:then_1
      (if (== Team2 _id)
        (return Team2)))
    (:then_2
      (return (select (Math|Random|RandomBool) Team2 Team1)))))

(fn FnGetNextOpponent
  (bind _id (Game|Bracket|FnGetPlayerTeamBracketID))
  (bind _bracketstatus (Variables|Game|Bracket|GetBracketStatus))
  (switch int (Math|Integer|%(Integer) _id 2) ; Odd or Even?
    (:0
      (LocalVariables|SetSearchTerm (.teamname (.Value (Utilities|Map|Find _bracketstatus (- _id 1))))))
    (:1
      (LocalVariables|SetSearchTerm (.teamname (.Value (Utilities|Map|Find _bracketstatus (+ _id 1)))))))
  (bind _outrownames (DataTable|GetDataTableRowNames "/Game/_AwfulJam18/Core/DT_Teams.DT_Teams"))
  (bind _array_element (Utilities|Array|ForEachLoopwithBreak _outrownames :!label _label)
    (:LoopBody
      (bind _returnvalue (Utilities|GetDataTableRow "/Game/_AwfulJam18/Core/DT_Teams.DT_Teams" _array_element)
        (:then
          (if (Utilities|Enum|Equal(Enum) (.teamName (Utilities|Struct|BreakS_Team _returnvalue)) (LocalVariables|GetSearchTerm))
            (LocalVariables|SetFoundOpponent _returnvalue)
            (goto _label Break)))))
    (:Completed
      (return (LocalVariables|GetFoundOpponent)))))

(fn FnProgresstoNextRound
  (bind _array (Utilities|Array|MakeArray 13 14))
  (Utilities|FlowControl|Sequence
    (:then_0
      (LocalVariables|Sett_PlayerBracketID (Game|Bracket|FnGetPlayerTeamBracketID)) ; For safety purposes
      (if (.ReturnValue (Utilities|Map|Find (Variables|Game|Bracket|GetBracketStatus) 9)) ; Are we moving to the finals now?
        (if (Utilities|Array|ContainsItem _array (Game|Bracket|FnGetPlayerTeamBracketID)) ; Is the player already in the finals? If so, we've just won the game!
          (CallFunction|EhonWontheTournament)
          (else
            (for _array_element _array
              (switch int _array_element
                (:13
                  (Game|Teams|FnAddTeamtoMatch _array_element (Game|Match|FnResolveMatch 9 10)))
                (:14
                  (Game|Teams|FnAddTeamtoMatch _array_element (Game|Match|FnResolveMatch 11 12)))))))
        (else
          (for _array_element_2 (Utilities|Array|MakeArray 9 10 11 12 13)
            (switch int _array_element_2
              (:9
                (Game|Teams|FnAddTeamtoMatch _array_element_2 (Game|Match|FnResolveMatch 1 2)))
              (:10
                (Game|Teams|FnAddTeamtoMatch _array_element_2 (Game|Match|FnResolveMatch 3 4)))
              (:11
                (Game|Teams|FnAddTeamtoMatch _array_element_2 (Game|Match|FnResolveMatch 5 6)))
              (:12
                (Game|Teams|FnAddTeamtoMatch _array_element_2 (Game|Match|FnResolveMatch 7 8))))))))
    (:then_1
      (LocalVariables|Sett_PlayerBracketID (Game|Bracket|FnGetPlayerTeamBracketID)) ; Update to the new BracketID now that we've updated the bracket
      (return))))

(fn FnAddTeamtoMatch
  (params (MatchSlotID :type Integer%20%28by%20ref%29) (TeamID :type Integer%20%28by%20ref%29))
  (bind _bracketstatus (Variables|Game|Bracket|GetBracketStatus))
  (Utilities|Map|Add _bracketstatus MatchSlotID (.Value (Utilities|Map|Find _bracketstatus TeamID)))
  (return))

(fn FnUnlockBreed
  (params (Breed :type S%20Dog%20Structure))
  (Utilities|Array|AddUnique (Variables|Game|Teams|GetUnlockedBreeds) Breed)
  (return))

(fn FnGameShowNotification
  (params (NotificationText :type Text))
  (bind _asbp_game_hud (Utilities|Casting|CastToBP_Game_HUD (HUD|GetHUD (Game|GetPlayerController 0))))
  (Default|EhonShowNotification (Variables|/Game/_AwfulJam18/Core/HUDs/BP_Game_HUD.BP_Game_HUD_C|GetUI_Gameplay _asbp_game_hud) NotificationText))

(fn FnGetPlayerTeamBracketID
  (bind _bracketstatus (Variables|Game|Bracket|GetBracketStatus))
  (Utilities|FlowControl|Sequence
    (:then_0
      (bind _keys (Utilities|Map|Keys _bracketstatus))
      (for _array_element _keys ; Figure out all of the instances where the player's team is in the bracket, such that we end up with the largest ID number!
        (if (and (.ReturnValue (Utilities|Map|Find _bracketstatus _array_element)) (Utilities|Enum|Equal(Enum) (.teamname (.Value (Utilities|Map|Find _bracketstatus _array_element))) (.teamname (Variables|Game|Teams|GetChosenTeam))))
          (if (< (LocalVariables|Gett_TempID) _array_element)
            (LocalVariables|Sett_TempID _array_element)))))
    (:then_1
      (return (LocalVariables|Gett_TempID)))))

(fn FnInitSaveGameData
  (Utilities|FlowControl|Sequence
    (:then_0
      (bind _returnvalue (SaveGame|DoesSaveGameExist (Variables|SaveGame|GetSaveGameSlot)))
      (if _returnvalue
        (bind _returnvalue_2 (SaveGame|LoadGamefromSlot (Variables|SaveGame|GetSaveGameSlot)))
        (bind _asbp_awful_jam_18_sg (Utilities|Casting|CastToBP_AwfulJam18_SG _returnvalue_2))
        (Variables|SaveGame|SetSaveGameData _asbp_awful_jam_18_sg)
        (Development|PrintString "SAVEGAME FOUND")
        (else
          (bind _returnvalue_3 (SaveGame|CreateSaveGameObject "/Game/_AwfulJam18/Core/BP_AwfulJam18_SG.BP_AwfulJam18_SG_C"))
          (Variables|SaveGame|SetSaveGameData _returnvalue_3)
          (Development|PrintString "NEW SAVEGAME CREATED"))))
    (:then_1
      (return))))

(fn FnReadSaveGameData
  (bind _savegamedata (Variables|SaveGame|GetSaveGameData)
    (:then
      (Utilities|FlowControl|Sequence
        (:then_0
          (Variables|Game|SetbHasBeatenTheGameBefore (Variables|/Game/_AwfulJam18/Core/BP_AwfulJam18_SG.BP_AwfulJam18_SG_C|GetbHasBeatenGameBefore _savegamedata)))
        (:then_2
          (return))))
    (:else)))

(fn FnWriteSaveGameData
  (bind _savegamedata (Variables|SaveGame|GetSaveGameData)
    (:then
      (Utilities|FlowControl|Sequence
        (:then_0
          (Utilities|FlowControl|Sequence
            (:then_0
              (Variables|/Game/_AwfulJam18/Core/BP_AwfulJam18_SG.BP_AwfulJam18_SG_C|SetbHasBeatenGameBefore _savegamedata (Variables|Game|GetbHasBeatenTheGameBefore)))))
        (:then_1
          (SaveGame|SaveGametoSlot _savegamedata (Variables|SaveGame|GetSaveGameSlot))
          (return))))
    (:else)))