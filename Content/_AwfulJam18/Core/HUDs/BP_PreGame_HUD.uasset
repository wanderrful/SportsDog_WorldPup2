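; Pre-game HUD that shows the WB_PreGame widget for the owning player.
; BeginPlay shows the mouse cursor, creates the widget, stores it and adds it to the viewport.
; EndPlay hides the cursor and removes the widget.
; A Game-and-UI input mode call focused on the widget is present but unconnected, so it never runs.
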(event EventBeginPlay
  (bind _playerowner (Variables|Default|GetPlayerOwner))
  (Variables|/Script/Engine.PlayerController|SetbShowMouseCursor _playerowner true)
  (bind _returnvalue (UserInterface|CreateWidget "/Game/_AwfulJam18/UI/WB_PreGame.WB_PreGame_C" _playerowner))
  (bind _output_get (Variables|Default|SetUI_PreGame _returnvalue))
  (UserInterface|Viewport|AddtoViewport _output_get 0))

(event EventEndPlay
  (params (EndPlayReason :type EEndPlayReason%20Enum :default "Destroyed"))
  (Variables|/Script/Engine.PlayerController|SetbShowMouseCursor (Variables|Default|GetPlayerOwner) false)
  (Widget|RemovefromParent (Variables|Default|GetUI_PreGame)))

(fn ConstructionScript)