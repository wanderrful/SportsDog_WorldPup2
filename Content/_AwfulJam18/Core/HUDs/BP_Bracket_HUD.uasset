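; BP_Bracket_HUD is the HUD that shows the between-match bracket screen or a game over screen.
; On BeginPlay it shows the mouse cursor and creates the bracket, win and lose widgets.
; Game instance flags for beating the game or being knocked out select which widget goes on screen, with the bracket as the default.
; EndPlay hides the cursor and removes all three widgets.
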(event EventBeginPlay
  (bind _playerowner (Variables|Default|GetPlayerOwner))
  (Variables|/Script/Engine.PlayerController|SetbShowMouseCursor _playerowner true)
  (bind _returnvalue (UserInterface|CreateWidget "/Game/_AwfulJam18/UI/WB_Bracket.WB_Bracket_C" _playerowner))
  (Variables|Default|SetUI_Bracket _returnvalue)
  (bind _returnvalue_2 (UserInterface|CreateWidget "/Game/_AwfulJam18/UI/WB_GameOver_Win.WB_GameOver_Win_C" (Variables|Default|GetPlayerOwner)))
  (Variables|Default|SetUI_GameOver_Win _returnvalue_2)
  (bind _returnvalue_3 (UserInterface|CreateWidget "/Game/_AwfulJam18/UI/WB_GameOver_Lose.WB_GameOver_Lose_C" (Variables|Default|GetPlayerOwner)))
  (Variables|Default|SetUI_GameOver_Lose _returnvalue_3)
  (bind _asbp_awful_jam_18_gi (Utilities|Casting|CastToBP_AwfulJam18_GI (Game|GetGameInstance)))
  (if (Variables|/Game/_AwfulJam18/Core/BP_AwfulJam18_GI.BP_AwfulJam18_GI_C|GetbJustBeatTheGame _asbp_awful_jam_18_gi) ; Should we show the Game Over (WIN) UI?
    (UserInterface|Viewport|AddtoViewport (Variables|Default|GetUI_GameOver_Win) 0)
    (elif (Variables|/Game/_AwfulJam18/Core/BP_AwfulJam18_GI.BP_AwfulJam18_GI_C|GetbWasKnockedOut _asbp_awful_jam_18_gi) ; Should we show the Game Over (LOSE) UI?
      (UserInterface|Viewport|AddtoViewport (Variables|Default|GetUI_GameOver_Lose) 0)
      (else
        (UserInterface|Viewport|AddtoViewport (Variables|Default|GetUI_Bracket) 0) ; Logically, we should just show the normal between-matches UI bracket
      ))))

(event EventEndPlay
  (params (EndPlayReason :type EEndPlayReason%20Enum :default "Destroyed"))
  (Variables|/Script/Engine.PlayerController|SetbShowMouseCursor (Variables|Default|GetPlayerOwner) false)
  (Widget|RemovefromParent (Variables|Default|GetUI_Bracket))
  (Widget|RemovefromParent (Variables|Default|GetUI_GameOver_Win))
  (Widget|RemovefromParent (Variables|Default|GetUI_GameOver_Lose)))

(fn ConstructionScript)