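; Match camera that follows the ball, switching between a sideline view and an end view behind either side of the pitch.
; On reset it returns home, finds the ball and blends in as player 0's view target.
; Tick swaps views by ball X with a hysteresis band, then eases position and look-at rotation, moving closer during penalty kicks.
; Cine camera focal length eases with ball distance and height.
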(event Custom|Reset
  ;[1 1 1] Reset
  (if (Variables|Default|Getenabled)
    (Actor|Tick|SetActorTickEnabled true)
    (Transformation|SetActorLocation (Variables|Default|GetHome%20Position) false true)
    (bind _outactors (Actor|GetAllActorsOfClass "/Game/_AwfulJam18/Ball/Ball.Ball_C"))
    (bind _output_get (Variables|Default|SetBall (Utilities|Array|Get(acopy) _outactors)))
    (Game|Player|SetViewTargetwithBlend (Game|GetPlayerController 0) self 1.0 "VTBlend_Linear" 0.0 false)
    (bind _ascine_camera_component (Utilities|Casting|CastToCineCameraComponent (Variables|CameraActor|GetCameraComponent)))
    (Variables|Default|SetCineCamera _ascine_camera_component)))

(event EventBeginPlay
  ;[1 1 1] Beginplay
  (bind _asbp_game_gm_match (Utilities|Casting|CastToBP_Game_GM_Match (Game|GetGameMode)))
  (Variables|Default|SetGameMode _asbp_game_gm_match)
  (Actor|Tick|SetActorTickEnabled false)
  (Variables|Default|SetHome%20Position (Transformation|GetActorLocation))
  (Utilities|FlowControl|Delay 0.1)
  (CallFunction|Reset))

(event Collision|EventActorBeginOverlap
  (params (OtherActor :type Actor%20Object%20Reference)))

(event EventTick
  (params (DeltaSeconds :type Float%20%28single-precision%29))
  (bind _returnvalue (Transformation|GetActorLocation))
  (bind _returnvalue_2 (Transformation|GetActorLocation))
  (bind _ball (Variables|Default|GetBall))
  (bind _ball_2 (Variables|Default|GetBall))
  (bind _cinecamera (Variables|Default|GetCineCamera))
  (bind _ball_3 (Variables|Default|GetBall))
  (bind _returnvalue_3 (Transformation|GetActorLocation _ball))
  (bind _returnvalue_4 (Transformation|GetActorLocation _ball_3))
  (bind _returnvalue_5 (Transformation|GetActorLocation _ball_2))
  (bind _returnvalue_6 (Math|Rotator|FindLookatRotation _returnvalue _returnvalue_3))
  (bind (_x _y _z) (Math|Vector|BreakVector _returnvalue_4))
  (bind _returnvalue_7 (Math|Float|Absolute(Float) (.x _returnvalue_5)))
  (bind _returnvalue_8 (+ _x 0.5))
  (bind _returnvalue_9 (Math|Float|Sign(Float) _returnvalue_8))
  (Variables|Default|SetdeltaSec DeltaSeconds)
  (Utilities|FlowControl|Sequence
    (:then_0
      (Utilities|FlowControl|Sequence
        (:then_0
          (if (and (!= (Variables|Default|GetcameraID) 1) (> _returnvalue_7 3e+03))
            (Transformation|SetActorLocation (Math|Vector|MakeVector (* (Math|Float|Sign(Float) (+ (.X (Math|Vector|BreakVector (Transformation|GetActorLocation (Variables|Default|GetBall)))) 0.5)) 6e+03) 0.0 7.5e+02) false false)
            (Transformation|SetActorRotation _returnvalue_6)
            (Variables|Default|SetcameraID 1)))
        (:then_1
          (if (and (!= (Variables|Default|GetcameraID) 0) (< _returnvalue_7 2e+03))
            (Transformation|SetActorLocation (Math|Vector|MakeVector (.X (Math|Vector|BreakVector (Transformation|GetActorLocation (Variables|Default|GetBall)))) -4e+03 2e+03) false false)
            (Transformation|SetActorRotation _returnvalue_6)
            (Variables|Default|SetcameraID 0)))))
    (:then_1
      (Variables|Default|SetDistanceToBall (Math|Vector|VectorLength (- (Transformation|GetActorLocation) (Transformation|GetActorLocation (Variables|Default|GetBall)))))
      (Utilities|FlowControl|Sequence
        (:then_0
          (switch int (Variables|Default|GetcameraID)
            (:0
              (Transformation|SetActorLocation (Math|Vector|MakeVector (Math|Interpolation|FInterpTo (.x _returnvalue_2) (.x (Transformation|GetActorLocation (Variables|Default|GetBall))) (Variables|Default|GetdeltaSec) 0.5) -4e+03 (.z _returnvalue_2)) false false))
            (:1
              (if (Variables|/Game/_AwfulJam18/Core/BP_Game_GM_Match.BP_Game_GM_Match_C|GetpenaltyKickActive (Variables|Default|GetGameMode))
                (Transformation|SetActorLocation (Math|Vector|MakeVector (* _returnvalue_9 3e+03) (Math|Interpolation|FInterpTo (.y (Transformation|GetActorLocation)) (.y (Transformation|GetActorLocation (Variables|Default|GetBall))) (Variables|Default|GetdeltaSec) 0.5) 6.5e+02) false false)
                (else
                  (Transformation|SetActorLocation (Math|Vector|MakeVector (* _returnvalue_9 6e+03) (Math|Interpolation|FInterpTo (.y (Transformation|GetActorLocation)) (.y (Transformation|GetActorLocation (Variables|Default|GetBall))) (Variables|Default|GetdeltaSec) 0.5) 6.5e+02) false false))))))
        (:then_1
          (Variables|/Script/CinematicCamera.CineCameraComponent|SetCurrentFocalLength _cinecamera (Math|Interpolation|FInterpTo (Variables|/Script/CinematicCamera.CineCameraComponent|GetCurrentFocalLength _cinecamera) (- (Math|Float|Clamp(Float) (/ (- (Variables|Default|GetDistanceToBall) 5e+02) 85.0) 15.0 6e+01) (/ _z 2e+02)) (Variables|Default|GetdeltaSec) 1.0))
          (Transformation|SetActorRotation (Math|Interpolation|RInterpTo (Transformation|GetActorRotation) (Math|Rotator|FindLookatRotation (Transformation|GetActorLocation) (Transformation|GetActorLocation (Variables|Default|GetBall))) (Variables|Default|GetdeltaSec) 4.0)))))))

(fn ConstructionScript)