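; Base character for AI soccer dogs, used in matches and pre-game, with breed-driven mesh, stats and voice.
; InitDog applies team shirt colors and a breed from the game instance or DT_Dogs; matches then start role-specific behavior trees, random barks and goal/assist tracking.
; Tick shifts the reach capsule along velocity and scales it by ball distance.
; Tackles ragdoll the mesh temporarily and drain stamina; exhaustion weakens stats and shows a marker.
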(event Custom|eh_OnGoalScored
  (params (GoalScoredBy :type BP%20Base%20Dog%20Object%20Reference) (GoalAssistedBy :type BP%20Base%20Dog%20Object%20Reference))
  (|OnGoalScoredGraph GoalScoredBy GoalAssistedBy))

(event Custom|Sound_Ruff
  ;[1 1 1] Ruff
  (switch name (Variables|Default|GetdogBreed)
    (:bernard
      (CallFunction|PlayDogSound "/Game/Sound/World_Pup_-_VO_edits/Dogs/DogLarge/VO_DogLarge_Ruff_Cue.VO_DogLarge_Ruff_Cue" :!label _label))
    (:husky
      (goto _label))
    (:shepherd
      (goto _label))
    (:samoyed
      (goto _label))
    (:shiba
      (CallFunction|PlayDogSound "/Game/Sound/World_Pup_-_VO_edits/Dogs/DogSmall/VO_DogSmall_Ruff_Cue.VO_DogSmall_Ruff_Cue" :!label _label_2))
    (:wiener
      (goto _label_2))
    (:corgi
      (goto _label_2))
    (:chihuahua
      (goto _label_2))))

(event Custom|PreGame_AIMoveTo
  (params (Goal :type Vector%20%28by%20ref%29))
  ;[1 1 1] PreGame AIMoveTo
  (AI|Navigation|SimpleMovetoLocation (AI|GetAIController self) Goal))

(event Custom|Sound_Bark
  ;[1 1 1] Bark
  (switch name (Variables|Default|GetdogBreed)
    (:bernard
      (CallFunction|PlayDogSound "/Game/Sound/World_Pup_-_VO_edits/Dogs/DogLarge/VO_DogLarge_Bark_Cue.VO_DogLarge_Bark_Cue" :!label _label))
    (:husky
      (goto _label))
    (:shepherd
      (goto _label))
    (:samoyed
      (goto _label))
    (:shiba
      (CallFunction|PlayDogSound "/Game/Sound/World_Pup_-_VO_edits/Dogs/DogSmall/VO_DogSmall_Bark_Cue.VO_DogSmall_Bark_Cue" :!label _label_2))
    (:wiener
      (goto _label_2))
    (:corgi
      (goto _label_2))
    (:chihuahua
      (goto _label_2))))

(event Custom|StaminaEdit
  (params (deltaStamina :type Integer))
  (Variables|Default|Setstamina (+ (Variables|Default|Getstamina) deltaStamina))
  (if (<= (Variables|Default|Getstamina) 0)
    (CallFunction|FnSetExhaustedStats)
    (Game|SpawnActorfromClass "/Game/_AwfulJam18/UI/MatchWidgets/BP_CombatTextActor.BP_CombatTextActor_C" (Math|Transform|MakeTransform (Transformation|GetActorLocation)) "Undefined" 0 "Exhausted!" "(R=1.000000,G=0.000000,B=0.015526,A=1.000000)" 0)
    (Development|SetHiddeninGame (Variables|Default|GetExhaustedSphere) false false)
    (elif (>= (Variables|Default|Getstamina) 100)
      (CallFunction|FnSetDefaultStats)
      (Development|SetHiddeninGame (Variables|Default|GetExhaustedSphere) true false))))

(event Custom|eh_ChangeBreed
  (params (NewBreed :type S%20Dog%20Structure))
  (if (not (Utilities|Text|TextIsEmpty (Utilities|Text|ToText(String) (.BreedName (Utilities|Struct|BreakS_Dog NewBreed))))) ; Validate the input!
    (Utilities|FlowControl|Sequence
      (:then_0
        ;[1 1 1] 1) Update the GI's BreedMap for this Doggy
        (bind _asbp_awful_jam_18_gi (Utilities|Casting|CastToBP_AwfulJam18_GI (Game|GetGameInstance)))
        (Utilities|Map|Add (Variables|/Game/_AwfulJam18/Core/BP_AwfulJam18_GI.BP_AwfulJam18_GI_C|GetChosenDogBreeds _asbp_awful_jam_18_gi) (Variables|0ASoccer|GetPlayerID) NewBreed)
        (Variables|Default|SetAssignedBreed NewBreed))
      (:then_1
        ;[1 1 1] 2) Load and reset this dog to use the new breed
        (CallFunction|FnSetDefaultStats)))))

(event Custom|Sound_Arf
  ;[1 1 1] Arf
  (switch name (Variables|Default|GetdogBreed)
    (:bernard
      (CallFunction|PlayDogSound "/Game/Sound/World_Pup_-_VO_edits/Dogs/DogLarge/VO_DogLarge_Arf_Cue.VO_DogLarge_Arf_Cue" :!label _label))
    (:husky
      (goto _label))
    (:shepherd
      (goto _label))
    (:samoyed
      (goto _label))
    (:shiba
      (CallFunction|PlayDogSound "/Game/Sound/World_Pup_-_VO_edits/Dogs/DogSmall/VO_DogSmall_Arf_Cue.VO_DogSmall_Arf_Cue" :!label _label_2))
    (:wiener
      (goto _label_2))
    (:corgi
      (goto _label_2))
    (:chihuahua
      (goto _label_2))))

(event Custom|Tackled
  (bind _charactermovement (Variables|Character|GetCharacterMovement))
  (bind _mesh (Variables|Character|GetMesh))
  ;[1 1 1] Tackled
  (CallFunction|SoundHowl)
  (Variables|Default|SetisDown true)
  (Physics|SetSimulatePhysics (Variables|Character|GetMesh) true)
  (Pawn|Components|CharacterMovement|DisableMovement _charactermovement)
  (Transformation|SetActorLocation "25000.000000,25000.000000, 0" false true)
  (Utilities|FlowControl|Delay 4.0)
  (Pawn|Components|CharacterMovement|SetMovementMode _charactermovement "MOVE_Walking" 0)
  (Physics|SetSimulatePhysics _mesh false)
  (Transformation|SetActorLocation (Math|Vector|ProjectVectorontoPlane (Transformation|GetWorldLocation _mesh) "0, 0,1.000000") false true)
  (Transformation|AttachComponentToComponent _mesh (Variables|Default|GetCapsuleComponent) "None" "SnapToTarget" "SnapToTarget" "SnapToTarget" false)
  (Transformation|SetRelativeTransform _mesh (Math|Transform|MakeTransform "0, 0,-90.000000" "0,-90.000000, 0" (Math|Conversions|ToVector(Float) (Variables|Default|GetdogMeshScale))) false true)
  (Utilities|FlowControl|Delay 0.0)
  (Character|Jump)
  (Variables|Default|SetisDown false)
  (CallFunction|StaminaEdit -10))

(event Custom|Sound_Howl
  ;[1 1 1] Howl
  (switch name (Variables|Default|GetdogBreed)
    (:bernard
      (CallFunction|PlayDogSound "/Game/Sound/World_Pup_-_VO_edits/Dogs/DogLarge/VO_DogLarge_Howl_Cue.VO_DogLarge_Howl_Cue" :!label _label))
    (:husky
      (goto _label))
    (:shepherd
      (goto _label))
    (:samoyed
      (goto _label))
    (:shiba
      (CallFunction|PlayDogSound "/Game/Sound/World_Pup_-_VO_edits/Dogs/DogSmall/VO_DogSmall_Howl_Cue.VO_DogSmall_Howl_Cue" :!label _label_2))
    (:wiener
      (goto _label_2))
    (:corgi
      (goto _label_2))
    (:chihuahua
      (goto _label_2))))

(event Custom|DogThings
  (bind _asbp_game_gm_match (Utilities|Casting|CastToBP_Game_GM_Match (Game|GetGameMode)) ; If this cast succeeds, we're in gameplay mode. If not, we're in pre-game.
    (:then
      (if (Variables|/Game/_AwfulJam18/Core/BP_Game_GM_Match.BP_Game_GM_Match_C|GetballInPlay _asbp_game_gm_match)
        (switch int (Math|Random|RandomIntegerinRange 0 3) :!label _label
          (:0
            (CallFunction|SoundBark))
          (:1
            (CallFunction|SoundRuff))
          (:2
            (CallFunction|SoundArf))
          (:3
            (CallFunction|SoundWoof)))))
    (:CastFailed
      (if (Variables|Default|GetbIsPreGame)
        (goto _label)))))

(event Custom|Sound_Woof
  ;[1 1 1] Woof
  (switch name (Variables|Default|GetdogBreed)
    (:bernard
      (CallFunction|PlayDogSound "/Game/Sound/World_Pup_-_VO_edits/Dogs/DogLarge/VO_DogLarge_Woof_Cue.VO_DogLarge_Woof_Cue" :!label _label))
    (:husky
      (goto _label))
    (:shepherd
      (goto _label))
    (:samoyed
      (goto _label))
    (:shiba
      (CallFunction|PlayDogSound "/Game/Sound/World_Pup_-_VO_edits/Dogs/DogSmall/VO_DogSmall_Woof_Cue.VO_DogSmall_Woof_Cue" :!label _label_2))
    (:wiener
      (goto _label_2))
    (:corgi
      (goto _label_2))
    (:chihuahua
      (goto _label_2))))

(event Custom|PlayDogSound
  (params (Sound :type Sound%20Base%20Object%20Reference))
  (bind _returnvalue (Transformation|GetActorLocation))
  (bind _returnvalue_2 (Math|Random|RandomFloatinRange 0.3 0.6))
  (Audio|PlaySoundatLocation Sound _returnvalue)
  (if (Math|Random|RandomBool)
    (Utilities|FlowControl|Delay _returnvalue_2)
    (Audio|PlaySoundatLocation Sound _returnvalue)
    (if (Math|Random|RandomBool)
      (Utilities|FlowControl|Delay _returnvalue_2)
      (Audio|PlaySoundatLocation Sound _returnvalue))))

(event EventBeginPlay
  (bind _self self)
  (bind _returnvalue (AI|GetAIController _self))
  (|CallParentFunction)
  (Variables|Default|SetbIsPreGame (not (.bSuccess (Utilities|Casting|CastToBP_Game_GM_Match (Game|GetGameMode)))))
  (|InitDog
    (:NewParam2
      (if (not (Variables|Default|GetbIsPreGame))
        (Utilities|FlowControl|Sequence
          (:then_0
            (Utilities|FlowControl|Delay 0.2)
            (bind _asbp_game_gm_match (Utilities|Casting|CastToBP_Game_GM_Match (Game|GetGameMode)))
            (Utilities|IsValid (Variables|/Game/_AwfulJam18/Core/BP_Game_GM_Match.BP_Game_GM_Match_C|GetSoccerBall _asbp_game_gm_match)
              (:Is%20Valid
                (Variables|Default|SetSoccerBall (Variables|/Game/_AwfulJam18/Core/BP_Game_GM_Match.BP_Game_GM_Match_C|GetSoccerBall _asbp_game_gm_match)))))
          (:then_1
            (switch Utilities|FlowControl|Switch|SwitchonPlayerRole (Variables|0ASoccer|GetplayerRole)
              (:NewEnumerator0
                (AI|RunBehaviorTree _returnvalue "/Game/_AwfulJam18/Core/AI/BT_Goalkeeper.BT_Goalkeeper"))
              (:NewEnumerator3
                (AI|RunBehaviorTree _returnvalue "/Game/_AwfulJam18/Core/AI/BT_PlayerDog.BT_PlayerDog"))))
          (:then_2
            (bind _asbp_game_gs (Utilities|Casting|CastToBP_Game_GS (Game|GetGameState))) ; (Love) Create event bindings to increment the goal/assist variables for this dog!
            (EventDispatchers|BindEventtoEdGoalScored _asbp_game_gs (delegate Custom|eh_OnGoalScored)))
          (:then_3
            (Utilities|Time|SetTimerbyEvent (delegate Custom|DogThings) (Math|Random|RandomFloatinRange 1.0 7.0) true)))))))

(event EventTick
  (params (DeltaSeconds :type Float%20%28single-precision%29))
  (bind _returnvalue (Transformation|GetActorLocation))
  (bind _soccerball (Variables|Default|GetSoccerBall))
  (|CallParentFunction DeltaSeconds)
  ;[1 1 1] Set Reach Capsule Size
  (if (not (or (not (Utilities|IsValid _soccerball)) (Variables|Default|GetbIsPreGame)))
    (Transformation|SetWorldTransform (Variables|Default|GetReach%20Capsule) (Math|Transform|MakeTransform (Math|Vector|Lerp(Vector) _returnvalue (+ _returnvalue (/ (Transformation|GetVelocity) 2.0)) 0.25) (Transformation|GetWorldRotation (Variables|Default|GetReach%20Capsule)) (Math|Vector|ClampVectorSize (Math|Conversions|ToVector(Float) (* (+ (* (Math|Vector|VectorLength (- (Transformation|GetWorldLocation (Variables|/Script/Engine.StaticMeshActor|GetStaticMeshComponent _soccerball)) (Transformation|GetActorLocation))) 0.25) 1e+02) 0.005)) 1.5 5.0)) false false)))

(fn ConstructionScript
  (|CallParentFunction)
  (Utilities|FlowControl|Sequence
    (:then_0
      (if (== (Variables|0ASoccer|GetTeamID) 0)
        (Variables|Default|SetTags (Utilities|Array|MakeArray "Team1"))
        (else
          (Variables|Default|SetTags (Utilities|Array|MakeArray "Team2")))))))

(fn FnGetBreed
  (bind _asbp_awful_jam_18_gi (Utilities|Casting|CastToBP_AwfulJam18_GI (Game|GetGameInstance))
    (:then
      (bind _returnvalue (Utilities|GetDataTableRow "/Game/_AwfulJam18/Core/DT_Dogs.DT_Dogs" (.dog (Variables|/Game/_AwfulJam18/Core/BP_AwfulJam18_GI.BP_AwfulJam18_GI_C|GetChosenTeam _asbp_awful_jam_18_gi)))
        (:then
          (if (Variables|Default|GetbIsPreGame) ; Are we in PreGame mode?
            (return _returnvalue)
            (elif (.ReturnValue (Utilities|Map|Find (Variables|/Game/_AwfulJam18/Core/BP_AwfulJam18_GI.BP_AwfulJam18_GI_C|GetChosenDogBreeds _asbp_awful_jam_18_gi) (Variables|0ASoccer|GetPlayerID)))
              (Utilities|IsValid (.Mesh (Utilities|Struct|BreakS_Dog (.Value (Utilities|Map|Find (Variables|/Game/_AwfulJam18/Core/BP_AwfulJam18_GI.BP_AwfulJam18_GI_C|GetChosenDogBreeds _asbp_awful_jam_18_gi) (Variables|0ASoccer|GetPlayerID))))) ; This is just quick way to check that the given breed won't cause an invisibility glitch
                (:Is%20Valid
                  (return (.Value (Utilities|Map|Find (Variables|/Game/_AwfulJam18/Core/BP_AwfulJam18_GI.BP_AwfulJam18_GI_C|GetChosenDogBreeds _asbp_awful_jam_18_gi) (Variables|0ASoccer|GetPlayerID)))))
                (:Is%20Not%20Valid
                  _)))))
        (:RowNotFound
          _)))
    (:CastFailed
      _))
  (bind _returnvalue_2 (Utilities|GetDataTableRow "/Game/_AwfulJam18/Core/DT_Dogs.DT_Dogs" (select (Utilities|Text|TextIsEmpty (Utilities|Text|ToText(Name) (.dog (Variables|/Game/_AwfulJam18/Core/BP_AwfulJam18_GI.BP_AwfulJam18_GI_C|GetCurrentOpposingTeam _asbp_awful_jam_18_gi)))) (Utilities|Name|MakeLiteralName "bernard") (.dog (Variables|/Game/_AwfulJam18/Core/BP_AwfulJam18_GI.BP_AwfulJam18_GI_C|GetCurrentOpposingTeam _asbp_awful_jam_18_gi)))) ; This dog logically must be on the opposing team!
    (:then
      (return _returnvalue_2))
    (:RowNotFound
      (bind _returnvalue_3 (Utilities|GetDataTableRow "/Game/_AwfulJam18/Core/DT_Dogs.DT_Dogs" "retriever")
        (:then
          (return _returnvalue_3) ; Invalid dog breed specified! Assume bernard by default
        )))))

(fn FnGetHomePosition
  (bind _returnvalue (Transformation|GetActorLocation))
  (bind (_x _y _z) (Math|Vector|BreakVector _returnvalue))
  (if (Variables|Default|GetbIsPreGame) ; Are we in PreGame mode?
    (return (Math|Vector|MakeVector _x _y _z))
    (else
      (bind _asbp_awful_jam_18_gi (Utilities|Casting|CastToBP_AwfulJam18_GI (Game|GetGameInstance))
        (:then
          (if (== (Variables|0ASoccer|GetTeamID) 0) ; Is this dog on the Player's Team (0)?
            (if (.ReturnValue (Utilities|Map|Find (Variables|/Game/_AwfulJam18/Core/BP_AwfulJam18_GI.BP_AwfulJam18_GI_C|GetChosenStartingPositions _asbp_awful_jam_18_gi) (Variables|0ASoccer|GetPlayerID)))
              (return (Math|Vector|MakeVector (.x (.Value (Utilities|Map|Find (Variables|/Game/_AwfulJam18/Core/BP_AwfulJam18_GI.BP_AwfulJam18_GI_C|GetChosenStartingPositions _asbp_awful_jam_18_gi) (Variables|0ASoccer|GetPlayerID)))) (.y (.Value (Utilities|Map|Find (Variables|/Game/_AwfulJam18/Core/BP_AwfulJam18_GI.BP_AwfulJam18_GI_C|GetChosenStartingPositions _asbp_awful_jam_18_gi) (Variables|0ASoccer|GetPlayerID)))) _z))
              (else
                (return (Math|Vector|MakeVector _x _y _z))))))
        (:CastFailed
          (return (Math|Vector|MakeVector _x _y _z)))))))

(fn FnSetDefaultStats
  (bind _assignedbreed (Variables|Default|GetAssignedBreed))
  (bind _charactermovement (Variables|Character|GetCharacterMovement))
  (bind _mesh (Variables|Character|GetMesh))
  (Utilities|FlowControl|Sequence
    (:then_0
      (Variables|Default|SetdogMeshScale (.meshscale _assignedbreed))
      (Variables|/Script/Engine.CharacterMovementComponent|SetMaxWalkSpeed _charactermovement (+ (Math|Float|MakeLiteralFloat 3.5e+02) (Math|Conversions|ToFloat(Integer) (* (.speed _assignedbreed) 8)))))
    (:then_1
      (Variables|Default|SettackleStrength (.strength _assignedbreed)))
    (:then_2
      (Variables|/Script/Engine.CharacterMovementComponent|SetMaxAcceleration _charactermovement (+ (Math|Float|MakeLiteralFloat 7e+02) (Math|Conversions|ToFloat(Integer) (* (.agility _assignedbreed) 10)))))
    (:then_3
      (Class|SkinnedMeshComponent|SetSkeletalMesh _mesh (.mesh _assignedbreed) true)
      (Components|SkeletalMesh|SetAnimInstanceClass _mesh (.animbp _assignedbreed))
      (Transformation|SetRelativeScale3D _mesh (Math|Conversions|ToVector(Float) (.meshscale _assignedbreed)))
      (Components|Capsule|SetCapsuleSize (Variables|Default|GetCapsuleComponent) (* (.meshscale _assignedbreed) 2.5e+02) 9e+01 true)
      (Variables|Default|SetdogBreed (.breedkey _assignedbreed)) ; For compatibility purposes -Love
    )
    (:then_4
      (Variables|Default|SetkickStat (.kick _assignedbreed)))
    (:then_5
      (Variables|Default|SetpassStat (.pass _assignedbreed)))
    (:then_6
      (Variables|Default|Setstamina (.stamina _assignedbreed)))
    (:then_7
      (Variables|Default|SetGoalKeeping (.goalkeeping _assignedbreed)))))

(fn FnSetExhaustedStats
  (bind _assignedbreed (Variables|Default|GetAssignedBreed))
  (bind _charactermovement (Variables|Character|GetCharacterMovement))
  (bind _mesh (Variables|Character|GetMesh))
  (Utilities|FlowControl|Sequence
    (:then_0
      (Variables|Default|SetdogMeshScale (.meshscale _assignedbreed))
      (Variables|/Script/Engine.CharacterMovementComponent|SetMaxWalkSpeed _charactermovement (+ (Math|Float|MakeLiteralFloat 0.0) (Math|Conversions|ToFloat(Integer) (* (.speed _assignedbreed) 6)))))
    (:then_1
      (Variables|Default|SettackleStrength (/ (.strength _assignedbreed) 2)))
    (:then_2
      (Variables|/Script/Engine.CharacterMovementComponent|SetMaxAcceleration _charactermovement (+ (Math|Float|MakeLiteralFloat 0.0) (Math|Conversions|ToFloat(Integer) (* (.agility _assignedbreed) 8)))))
    (:then_3
      (Class|SkinnedMeshComponent|SetSkeletalMesh _mesh (.mesh _assignedbreed) true)
      (Transformation|SetRelativeScale3D _mesh (Math|Conversions|ToVector(Float) (.meshscale _assignedbreed)))
      (Components|SkeletalMesh|SetAnimInstanceClass _mesh "/Game/_AwfulJam18/Characters/Bernard/ABP_Bernard.ABP_Bernard_C")
      (Components|Capsule|SetCapsuleSize (Variables|Default|GetCapsuleComponent) (* (.meshscale _assignedbreed) 3e+02) 9e+01 true)
      (Variables|Default|SetdogBreed (.breedkey _assignedbreed)) ; For compatibility purposes -Love
    )
    (:then_4
      (Variables|Default|SetkickStat (/ (.kick _assignedbreed) 2)))
    (:then_5
      (Variables|Default|SetpassStat (/ (.pass _assignedbreed) 2)))
    (:then_6
      (Variables|Default|Setstamina 0))
    (:then_7
      (Variables|Default|SetGoalKeeping (/ (.goalkeeping _assignedbreed) 2)))))